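; Missile launcher Blueprint that spawns BP_Missile at its projectile location, with a fire cooldown and reserve ammo.
; LaunchMissile checks ammo and the Fire flag, spawns the missile, then starts a looping timer whose FireRate_E event re-enables Fire.
; AmmoCountFunc decrements the loaded count and refills up to three from TotalMissiles when empty.
; A separate Ready For Fire? macro implements a Delay-loop countdown, unused by the event graph.
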(event Custom|FireRate_E
  (Variables|Default|SetFire? true))

(event EventTick
  (params (DeltaSeconds :type Float%20%28single-precision%29)))

(event EventLaunchMissile
  (if (and (== 0 (Variables|Default|GetTotal%20Missiles)) (== 0 (Variables|Default|GetMissile)))
    (Development|PrintString "No Ammo")
    (elif (Variables|Default|GetFire?)
      (Game|SpawnActorfromClass "/Game/Guns/Projectile/Missile/BP_Missile.BP_Missile_C" (Transformation|GetWorldTransform (Variables|Default|GetProjectile%20Locaiton%20)) "AlwaysSpawn" 0 0)
      (Development|PrintString (Utilities|String|Append (Utilities|String|ToString(Integer) (Variables|Default|GetTotal%20Missiles)) "/" (Utilities|String|ToString(Integer) (Variables|Default|GetMissile))))
      (CallFunction|AmmoCountFunc)
      (Variables|Default|SetFire? false)
      (Utilities|Time|SetTimerbyFunctionName 0 "FireRate_E" 5.0 true 5.0))))

(fn ConstructionScript)

(fn AmmoCountFunc
  (Variables|Default|SetMissile (- (Variables|Default|GetMissile) 1))
  (if (and (== (Variables|Default|GetMissile) 0) (> (Variables|Default|GetTotal%20Missiles) 0))
    (if (< (Variables|Default|GetTotal%20Missiles) 3)
      (Variables|Default|SetMissile (Variables|Default|GetTotal%20Missiles))
      (Variables|Default|SetTotal%20Missiles 0)
      (if (and (== (Variables|Default|GetMissile) 0) (== (Variables|Default|GetTotal%20Missiles) 0))
        (Variables|Default|SetMissile 0)
        (Variables|Default|SetTotal%20Missiles 0)
        (Development|PrintString "No Ammo"))
      (elif (> (Variables|Default|GetTotal%20Missiles) 3)
        (bind _output_get (Variables|Default|SetMissile 3))
        (Variables|Default|SetTotal%20Missiles (- (Variables|Default|GetTotal%20Missiles) _output_get))))))