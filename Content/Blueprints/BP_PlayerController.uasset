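; Player controller Blueprint that swaps the player's car for a chosen model at runtime.
; The EnumValue event takes a car type, saves the current pawn's transform and destroys that pawn.
; It then switches on the type to spawn the Beryllium, Chevrolate or Mustange Blueprint at that transform, print a message and possess the new pawn through player controller 0.
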(event EventBeginPlay)

(event EventTick
  (params (DeltaSeconds :type Float%20%28single-precision%29)))

(event EventEnumValue
  (params (Car%20Type :type E_CarSelection%20Enum :default "NewEnumerator0"))
  (Variables|Default|SetPlayer%20Start%20Location (Transformation|GetActorTransform (Pawn|GetControlledPawn (Game|GetPlayerController 0))))
  (Actor|DestroyActor (Pawn|GetControlledPawn (Game|GetPlayerController 0)))
  (switch Utilities|FlowControl|Switch|SwitchonE_CarSelection Car%20Type
    (:NewEnumerator0
      (Development|PrintString "Beryllium Is New Pawn")
      (bind _returnvalue (Game|SpawnActorfromClass "/Game/BP_Beryllium.BP_Beryllium_C" (Variables|Default|GetPlayer%20Start%20Location) "Undefined" 0 0))
      (Pawn|Possess (Game|GetPlayerController 0) _returnvalue))
    (:NewEnumerator1
      (Development|PrintString "Chevrolate Is New Pawn")
      (bind _returnvalue_2 (Game|SpawnActorfromClass "/Game/BP_Chevrolate.BP_Chevrolate_C" (Variables|Default|GetPlayer%20Start%20Location) "Undefined" 0 0))
      (Pawn|Possess (Game|GetPlayerController 0) _returnvalue_2))
    (:NewEnumerator2
      (Development|PrintString "Mustang Is New Pawn")
      (bind _returnvalue_3 (Game|SpawnActorfromClass "/Game/BP_Mustange.BP_Mustange_C" (Variables|Default|GetPlayer%20Start%20Location) "Undefined" 0 0))
      (Pawn|Possess (Game|GetPlayerController 0) _returnvalue_3))))

(fn ConstructionScript)