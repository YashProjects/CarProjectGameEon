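; AI enemy car that drives at constant throttle with random steering jitter, issues an AI move toward the player, and dies when health runs out.
; On BeginPlay it spawns an attached head gun, yawed toward the player each Tick.
; Sphere hits and player overlaps play a shot and send damage; Tick re-arms a looping damage timer while the player is in range.
; Spline path-steering logic exists but never runs.
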(event OnComponentBeginOverlap(Sphere)
  (params (OverlappedComponent :type Primitive%20Component%20Object%20Reference) (OtherActor :type Actor%20Object%20Reference) (OtherComp :type Primitive%20Component%20Object%20Reference) (OtherBodyIndex :type Integer) (bFromSweep :type Boolean) (SweepResult :type Hit%20Result%20Structure%20%28by%20ref%29))
  ;[1 1 1] Call Damage Event Player Pawn
  (Utilities|IsValid OtherActor
    (:Is%20Valid
      (if (== OtherActor (Game|Player|GetPlayerPawn 0))
        (Variables|Default|SetPlayer%20In%20Range true)
        (Audio|PlaySoundatLocation "/Game/Sound/Sounds/GunShot/AR_Shot_1.AR_Shot_1" (Transformation|GetActorLocation) "0, 0, 0" 1.0 1.0 0.0 0 0 0)
        (Class|BPIHealth|HealthReduce(Message) OtherActor)))))

(event OnComponentEndOverlap(Sphere)
  (params (OverlappedComponent :type Primitive%20Component%20Object%20Reference) (OtherActor :type Actor%20Object%20Reference) (OtherComp :type Primitive%20Component%20Object%20Reference) (OtherBodyIndex :type Integer))
  ;[1 1 1] Call Damage Event Player Pawn
  (Utilities|IsValid OtherActor
    (:Is%20Valid
      (if (== OtherActor (Game|Player|GetPlayerPawn 0))
        (Variables|Default|SetPlayer%20In%20Range false)))))

(event OnComponentHit(Sphere)
  (params (HitComponent :type Primitive%20Component%20Object%20Reference) (OtherActor :type Actor%20Object%20Reference) (OtherComp :type Primitive%20Component%20Object%20Reference) (NormalImpulse :type Vector :default "0, 0, 0") (Hit :type Hit%20Result%20Structure%20%28by%20ref%29))
  ;[1 1 1] Call Damage Event Player Pawn
  (Audio|PlaySoundatLocation "/Game/Sound/Sounds/GunShot/AR_Shot_1.AR_Shot_1" (Transformation|GetActorLocation) "0, 0, 0" 1.0 1.0 0.0 0 0 0)
  (Class|BPIHealth|HealthReduce(Message) (stale OnComponentBeginOverlap(Sphere) OtherActor)))

(event Custom|Call%20Player%20Controller%20Damege
  ;[1 1 1] Call Damage Event Player Pawn
  (Audio|PlaySoundatLocation "/Game/Sound/Sounds/GunShot/AR_Shot_1.AR_Shot_1" (Transformation|GetActorLocation) "0, 0, 0" 1.0 1.0 0.0 0 0 0)
  (Class|BPIHealth|HealthReduce(Message) (stale OnComponentBeginOverlap(Sphere) OtherActor)))

(event Custom|Turret%20Rotation
  (bind _ai_headgun (Variables|Default|GetAI%20HeadGun))
  (bind _gun (Variables|/Game/AI/BP_AIHeadGun.BP_AIHeadGun_C|GetGun _ai_headgun))
  (bind _returnvalue (Transformation|GetWorldRotation _gun))
  ;[1 1 1] Turret Rotation
  (Utilities|IsValid _ai_headgun
    (:Is%20Valid
      (Transformation|SetWorldRotation _gun (Math|Rotator|MakeRotator (.roll _returnvalue) (.pitch _returnvalue) (Math|Float|Lerp (.yaw _returnvalue) (.yaw (Math|Rotator|FindLookatRotation (Transformation|GetWorldLocation _gun) (Transformation|GetActorLocation (Game|GetPlayerController 0)))) 0.5)) false false))))

(event EventDamageHealth
  (bind _ai_headgun (Variables|Default|GetAI%20HeadGun))
  ;[1 1 1] After Bullet Hit / Apply Damage
  (Variables|Default|SetHealth (- (Variables|Default|GetHealth) 0.04))
  (if (<= (Variables|Default|GetHealth) 0.0)
    (Actor|DestroyActor)
    (Utilities|IsValid _ai_headgun
      (:Is%20Valid
        (Actor|DestroyActor _ai_headgun)))))

(event EventTick
  (params (DeltaSeconds :type Float%20%28single-precision%29))
  (bind _vehiclemovement (Variables|Default|GetVehicleMovement))
  ;[1 1 1] AI Move & Steering
  (Utilities|FlowControl|Sequence
    (:then_0
      (bind _outactors (Actor|GetAllActorsOfClass "/Game/AI/BP_Path.BP_Path_C"))
      (Class|WheeledVehicleMovementComponent|SetSteeringInput _vehiclemovement (Math|Random|RandomFloatinRange -0.2 0.2))
      (Class|WheeledVehicleMovementComponent|SetThrottleInput _vehiclemovement 0.5))
    (:then_1
      (if (Variables|Default|GetPlayer%20In%20Range)
        (Utilities|Time|SetTimerbyEvent (delegate Custom|Call%20Player%20Controller%20Damege) 2.0 true)))
    (:then_2
      ;[1 1 1] Turret Rotate
      (CallFunction|TurretRotation))))

(event EventBeginPlay
  (bind _returnvalue (Game|GetPlayerController 0))
  ;[1 1 1] AI Move & Steering
  (Utilities|FlowControl|Sequence
    (:then_0
      (Class|WheeledVehicleMovementComponent|SetThrottleInput (Variables|Default|GetVehicleMovement) 0.5))
    (:then_1
      (AI|AIMoveTo self (Transformation|GetActorLocation _returnvalue) _returnvalue 5e+03 false
        (:OnFail
          (Development|PrintString "AI Move Fail"))))
    (:then_2
      ;[1 1 1] Spawn AI Turret
      (bind _returnvalue_2 (Game|SpawnActorfromClass "/Game/AI/BP_AIHeadGun.BP_AIHeadGun_C" (Transformation|GetWorldTransform (Variables|Default|GetProjectile%20Location)) "AlwaysSpawn" 0 0))
      (Variables|Default|SetAI%20HeadGun _returnvalue_2)
      (Transformation|AttachComponentToComponent _returnvalue_2 (Variables|Character|GetMesh) "None" "SnapToTarget" "SnapToTarget" "SnapToTarget" true))))

(fn ConstructionScript)

(fn GetPath
  (params (Splines :type Array%20of%20BP%20Path%20Object%20References))
  (bind _returnvalue (Transformation|GetActorLocation))
  (bind _output (Utilities|Array|Get(acopy) Splines))
  (bind _spline (Variables|/Game/AI/BP_Path.BP_Path_C|GetSpline _output))
  (return (Math|Float|MapRangeClamped (.yaw (Math|Rotator|Delta(Rotator) (Math|Rotator|FindLookatRotation _returnvalue (Spline|FindLocationClosesttoWorldLocation _spline (+ (* (Math|Vector|Normalize (Class|SplineComponent|FindTangentClosesttoWorldLocation _spline _returnvalue "World")) 5e+02) _returnvalue) "World")) (Transformation|GetActorRotation))) -9e+01 9e+01 -1.0 1.0)))