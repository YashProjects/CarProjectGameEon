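; BP_Zombie is a zombie enemy actor whose only working logic is taking damage.
; Each DamageHealth call subtracts a small fixed amount from Health and destroys the actor once it reaches zero.
; Chase and melee attack logic (move to player, distance-checked montage, player health message) is left unconnected and never runs, and Tick and BeginPlay are empty.
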(event EventDamageHealth
  ;[1 1 1] After Bullet Hit / Apply Damage
  (Variables|Default|SetHealth (- (Variables|Default|GetHealth) 0.04))
  (if (<= (Variables|Default|GetHealth) 0.0)
    (Actor|DestroyActor)))

(event Collision|EventActorBeginOverlap
  (params (OtherActor :type Actor%20Object%20Reference)))

(event EventBeginPlay)

(event EventTick
  (params (DeltaSeconds :type Float%20%28single-precision%29))
  ;[1 1 1] Zombie Attack
)

(fn ConstructionScript)