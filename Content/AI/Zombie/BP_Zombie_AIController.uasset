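; Zombie AI controller that sends its pawn toward a target reported by AI perception.
; On a successful sense, it stores the actor as Target and issues a move-to, but only if that actor equals player controller 0 itself, rather than its pawn.
; Losing sight has no handling, and a second move-to that re-checks Target validity is left unwired.
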(event OnTargetPerceptionUpdated(AIPerception)
  (params (Actor :type Actor%20Object%20Reference) (Stimulus :type AI%20Stimulus%20Structure))
  (if (== Actor (Game|GetPlayerController 0))
    (if (.bSuccessfullySensed (Utilities|Struct|BreakAIStimulus Stimulus))
      (bind _output_get (Variables|Default|SetTarget Actor))
      (AI|Navigation|MovetoActor _output_get 5e+01 true true true 0))))

(event EventBeginPlay)

(event EventTick
  (params (DeltaSeconds :type Float%20%28single-precision%29)))

(fn ConstructionScript)