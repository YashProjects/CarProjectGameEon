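; Player combat car Blueprint (Mustang) with mountable head gun, twin miniguns and missile launcher, plus health and ammo pickups.
; Weapon events spawn and attach guns to mesh sockets or destroy them.
; Fire input triggers guns using the GameMode's weapon-selection UI flags, while missile input spawns projectiles directly; the auto-fire loop is disconnected.
; Tick rotates the head gun toward the deprojected mouse when scoped and refreshes ammo counters for UI.
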(event Custom|Update%20Ammo%20UI
  (bind _headgun (Variables|Default|GetHeadGun))
  (bind _minigunright (Variables|Default|GetMiniGunRight))
  (bind _mini_gun_left (Variables|Default|GetMini%20Gun%20Left))
  ;[1 1 1] Update Ammo Counter For UI
  (Utilities|IsValid (Variables|Default|GetHeadGun)
    (:Is%20Valid
      (Variables|Default|SetTotal%20Ammo%20HG (Variables|/Game/Guns/BP_HeadGun.BP_HeadGun_C|GetTotalAmmoHG _headgun))
      (Variables|Default|SetCurret%20Ammo%20HG (Variables|/Game/Guns/BP_HeadGun.BP_HeadGun_C|GetAmmoHG _headgun)))
    (:Is%20Not%20Valid
      _))
  (Utilities|IsValid _minigunright
    (:Is%20Valid
      (Utilities|IsValid _mini_gun_left
        (:Is%20Valid
          (Variables|Default|SetTotal%20Ammo%20MG (+ (Variables|/Game/Guns/MiniGun/BP_MiniGun.BP_MiniGun_C|GetTotalAmmoMG _mini_gun_left) (Variables|/Game/Guns/MiniGun/BP_MiniGun.BP_MiniGun_C|GetTotalAmmoMG _minigunright)))
          (Variables|Default|SetCurret%20Ammo%20MG (+ (Variables|/Game/Guns/MiniGun/BP_MiniGun.BP_MiniGun_C|GetAmmoMG _minigunright) (Variables|/Game/Guns/MiniGun/BP_MiniGun.BP_MiniGun_C|GetAmmoMG _mini_gun_left))))))))

(event EventBeginPlay
  (Utilities|FlowControl|Sequence
    (:then_0
      ;[1 1 1] Car Move Sound
      (Utilities|FlowControl|Delay 1e+01)
      (if (> (Class|WheeledVehicleMovementComponent|GetEngineMaxRotationSpeed (Variables|Default|GetVehicleMovement)) 1e+01)
        (Audio|PlaySound2D "/Game/Sound/Sounds/Wav/Car_Move.Car_Move" 1.0 1.0 0.0 0 0)
        (else
          (Audio|PlaySound2D "/Game/Sound/Sounds/Wav/CopeLX_Gear_1.CopeLX_Gear_1" 1.0 1.0 0.0 0 0)))
      (Utilities|FlowControl|Delay 4.0))))

(event Collision|EventActorBeginOverlap
  (params (OtherActor :type Actor%20Object%20Reference)))

(event EventCrosshairRefon
  ;[1 1 1] Scope Mode On/Off
  (bind _asbp_hud (Utilities|Casting|CastToBP_HUD (HUD|GetHUD (Game|GetPlayerController 0))))
  (Variables|/Game/UI/UI_Crosshair.UI_Crosshair_C|SetCrosshair%20Visibility (Variables|/Game/UI/BP_HUD.BP_HUD_C|GetCrosshair%20UI _asbp_hud) "Visible"))

(event EventCrosshairRefOff
  ;[1 1 1] Scope Mode On/Off
  (Variables|/Game/UI/UI_Crosshair.UI_Crosshair_C|SetCrosshair%20Visibility (Variables|/Game/UI/BP_HUD.BP_HUD_C|GetCrosshair%20UI (stale EventCrosshairRefon _asbp_hud)) "Hidden"))

(event EventAmmoData
  (params (Ammo%20Data :type Struct%20Ammo%20Structure))
  (bind (_name _supportweapontype _mesh _ammotype _ammohold) (Utilities|Struct|BreakStruct_Ammo Ammo%20Data))
  (bind _headgun (Variables|Default|GetHeadGun))
  (bind _minigunright (Variables|Default|GetMiniGunRight))
  (bind _mini_gun_left (Variables|Default|GetMini%20Gun%20Left))
  (bind _missile_m (Variables|Default|GetMissile_M))
  ;[1 1 1] Ammo Added On Overlap
  (Development|PrintString "Ammo fucc Call")
  (switch Utilities|FlowControl|Switch|SwitchonE_Ammo _ammotype
    (:NewEnumerator0
      (Utilities|IsValid (Variables|Default|GetHeadGun)
        (:Is%20Valid
          (Variables|/Game/Guns/BP_HeadGun.BP_HeadGun_C|SetTotalAmmoHG _headgun (+ (Variables|/Game/Guns/BP_HeadGun.BP_HeadGun_C|GetTotalAmmoHG _headgun) _ammohold)))))
    (:NewEnumerator1
      (Utilities|IsValid (Variables|Default|GetMini%20Gun%20Left)
        (:Is%20Valid
          (Utilities|IsValid (Variables|Default|GetMiniGunRight)
            (:Is%20Valid
              (Variables|/Game/Guns/MiniGun/BP_MiniGun.BP_MiniGun_C|SetTotalAmmoMG _minigunright (+ _ammohold (Variables|/Game/Guns/MiniGun/BP_MiniGun.BP_MiniGun_C|GetTotalAmmoMG _minigunright)))
              (Variables|/Game/Guns/MiniGun/BP_MiniGun.BP_MiniGun_C|SetTotalAmmoMG _mini_gun_left (+ _ammohold (Variables|/Game/Guns/MiniGun/BP_MiniGun.BP_MiniGun_C|GetTotalAmmoMG _mini_gun_left))))))))
    (:NewEnumerator2
      (Utilities|IsValid (Variables|Default|GetMissile_M)
        (:Is%20Valid
          (Variables|/Game/Guns/Missile/BP_MissileLauncher.BP_MissileLauncher_C|SetTotal%20Missiles _missile_m (+ _ammohold (Variables|/Game/Guns/Missile/BP_MissileLauncher.BP_MissileLauncher_C|GetTotal%20Missiles _missile_m))))))))

(event EventHealthPack
  ;[1 1 1] Health Pack
  (Variables|Default|SetHealth (+ (Variables|Default|GetHealth) 0.25))
  (if (>= (Variables|Default|GetHealth) 1.0)
    (Variables|Default|SetHealth 1.0)))

(event EventHealthReduce
  ;[1 1 1] Apply Damage
  (bind _output_get (Variables|Default|SetHealth (- (Variables|Default|GetHealth) 0.06)))
  (if (<= (Variables|Default|GetHealth) 0.0)
    (Development|PrintString "Player Died By AI")
    (else
      (Development|PrintString (Utilities|String|ToString(Float) _output_get)))))

(event EventSpawnGun
  (params (Spawn :type Boolean))
  ;[1 1 1] HeadGun
  (bind _output_get (Variables|Default|SetSpawn%20HG Spawn))
  (Utilities|SpawnHeadGun _output_get))

(event EventTick
  (params (DeltaSeconds :type Float%20%28single-precision%29))
  (Utilities|FlowControl|Sequence
    (:then_0
      ;[1 1 1] Turret Movement
      (if (not (Math|Boolean|ANDBoolean (Variables|Default|GetSpawned?%20D%20HG) (not (Variables|Default|GetSpawn%20HG)) (Variables|Default|GetFire%20Control%20Head%20Gun)))
        (|RotateTurret (Variables|Default|GetScopeValue self) (Variables|Default|GetSpawn%20HG) (Utilities|IsValid (Variables|Default|GetHeadGun)))))
    (:then_1)
    (:then_2
      ;[1 1 1] Update UI
      (CallFunction|UpdateAmmoUI))))

(event EventDestroyActor
  (params (Spawned? :type Boolean))
  (bind _headgun (Variables|Default|GetHeadGun))
  ;[1 1 1] HeadGun
  (Variables|Default|SetSpawned?%20D%20HG Spawned?)
  (Utilities|IsValid _headgun
    (:Is%20Valid
      (Actor|DestroyActor _headgun))
    (:Is%20Not%20Valid
      (Development|PrintString "Something Went Wrong..!"))))

(event EventSpawnMiniGun
  (params (MiniGun :type Boolean))
  ;[1 1 1] MiniGun
  (bind _output_get (Variables|Default|SetMini%20Gun MiniGun))
  (Utilities|SpawnMiniGuns _output_get))

(event EventDestroyMiniGun
  (params (MiniGun%20D :type Boolean))
  (bind _mini_gun_left (Variables|Default|GetMini%20Gun%20Left))
  (bind _minigunright (Variables|Default|GetMiniGunRight))
  ;[1 1 1] MiniGun
  (Variables|Default|SetMini%20Gun%20D MiniGun%20D)
  (if (and (Utilities|IsValid _minigunright) (Utilities|IsValid _mini_gun_left))
    (Actor|DestroyActor _mini_gun_left)
    (Actor|DestroyActor _minigunright)
    (else
      (Development|PrintString "Something Went Wrong ..!"))))

(event EventSpawnMissile
  (params (Missile :type Boolean))
  ;[1 1 1] Missile
  (bind _output_get (Variables|Default|SetMissile Missile))
  (Utilities|SpawnMissileM _output_get))

(event EventDestroyMissile
  (params (Missile%20D :type Boolean))
  (bind _missile_m (Variables|Default|GetMissile_M))
  ;[1 1 1] Missile
  (Variables|Default|SetMissile%20D Missile%20D)
  (Utilities|IsValid _missile_m
    (:Is%20Valid
      (Actor|DestroyActor _missile_m))
    (:Is%20Not%20Valid
      (Development|PrintString "Something Went Wrong ..!"))))

(event EventFireButton
  ;[1 1 1] Fire
  (Variables|Default|SetAuto%20Fire%20On true)
  (Audio|PlaySound2D "/Game/Sound/Sounds/GunShot/AR_Shot_1.AR_Shot_1" 1.0 1.0 0.0 0 0)
  (|FireSystem))

(event Input|ActionEvents|InputActionFire
  (params (Key :type Key%20Structure :default "None"))
  ;[1 1 1] Fire
  (:Pressed
    (Variables|Default|SetAuto%20Fire%20On true)
    (Audio|PlaySound2D "/Game/Sound/Sounds/GunShot/AR_Shot_1.AR_Shot_1" 1.0 1.0 0.0 0 0)
    (|FireSystem))
  (:Released
    (Variables|Default|SetAuto%20Fire%20On false)))

(event Input|ActionEvents|InputActionMissileFire
  (params (Key :type Key%20Structure :default "None"))
  (bind _missile_m (Variables|Default|GetMissile_M))
  ;[1 1 1] Missile Launch
  (:Pressed
    (Utilities|IsValid _missile_m
      (:Is%20Valid
        (Audio|PlaySound2D "/Game/Sound/Sounds/GunShot/AR_Shot_1.AR_Shot_1" 1.0 1.0 0.0 0 0)
        (Game|SpawnActorfromClass "/Game/Guns/Projectile/Missile/BP_Missile.BP_Missile_C" (Transformation|GetWorldTransform (Variables|/Game/Guns/Missile/BP_MissileLauncher.BP_MissileLauncher_C|GetProjectile%20Locaiton%20 _missile_m)) "AlwaysSpawn" 0 0)))))

(event Input|ActionEvents|InputActionNitro
  (params (Key :type Key%20Structure :default "None"))
  ;[1 1 1] Apply Nitro
)

(fn ConstructionScript)

(fn RefHeadGun
  (return 0))

(fn HeadGunData
  (return 0 0))